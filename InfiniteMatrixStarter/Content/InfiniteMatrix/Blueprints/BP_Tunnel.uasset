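; Endless-tunnel segment with a rotating holed wall, a heal pack and an enemy.
; Passing its trigger zone has TunnelSpawner spawn another segment, destroys this one and adds player score.
; Overlaps drive player health: wall and enemy damage it, the pack restores it up to full, and bullets kill the enemy for points.
; Randomize functions, not called here, vary wall mesh and roll, plus pickup and enemy presence and offset.
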(event `self.ReceiveBeginPlay`)

(event `self.ReceiveTick`
  (params (DeltaSeconds :type "Float (single-precision)"))
  (`SceneComponent.K2_AddLocalRotation` (`self.WallMesh`) (`KismetMathLibrary.MakeRotator` (* DeltaSeconds (`self.RotateSpeed`))) false false))

(event `self.TriggerZone.OnComponentBeginOverlap`
  (params (OverlappedComponent :type "PrimitiveComponent Object Reference") (OtherActor :type "Actor Object Reference") (OtherComp :type "PrimitiveComponent Object Reference") (OtherBodyIndex :type Integer) (bFromSweep :type Boolean) (SweepResult :type "HitResult Structure (by ref)"))
  (bind _asbp_player (cast `/Game/InfiniteMatrix/Blueprints/BP_Player` OtherActor))
  (`/Game/InfiniteMatrix/Blueprints/BP_TunnelSpawner.SpawnTunnelAtSpawnPoint` (`self.TunnelSpawner`))
  (`self.K2_DestroyActor`)
  (bind _score (`/Game/InfiniteMatrix/Blueprints/BP_Player.Score` _asbp_player))
  (bind _returnvalue (+ _score 10.0))
  (set `/Game/InfiniteMatrix/Blueprints/BP_Player.Score` _returnvalue _asbp_player)
  (if (> _returnvalue (`/Game/InfiniteMatrix/Blueprints/BP_Player.HighScore` _asbp_player))
    (set `/Game/InfiniteMatrix/Blueprints/BP_Player.HighScore` _score _asbp_player)))

(event `self.WallMesh.OnComponentHit`
  (params (HitComponent :type "PrimitiveComponent Object Reference") (OtherActor :type "Actor Object Reference") (OtherComp :type "PrimitiveComponent Object Reference") (NormalImpulse :type "Vector Structure") (Hit :type "HitResult Structure (by ref)")))

(event `self.WallMesh.OnComponentBeginOverlap`
  (params (OverlappedComponent :type "PrimitiveComponent Object Reference") (OtherActor :type "Actor Object Reference") (OtherComp :type "PrimitiveComponent Object Reference") (OtherBodyIndex :type Integer) (bFromSweep :type Boolean) (SweepResult :type "HitResult Structure (by ref)"))
  (bind _asbp_player (cast `/Game/InfiniteMatrix/Blueprints/BP_Player` OtherActor))
  (set `/Game/InfiniteMatrix/Blueprints/BP_Player.Health` (- (`/Game/InfiniteMatrix/Blueprints/BP_Player.Health` _asbp_player) 0.5) _asbp_player))

(event `self.HealPack.OnComponentBeginOverlap`
  (params (OverlappedComponent :type "PrimitiveComponent Object Reference") (OtherActor :type "Actor Object Reference") (OtherComp :type "PrimitiveComponent Object Reference") (OtherBodyIndex :type Integer) (bFromSweep :type Boolean) (SweepResult :type "HitResult Structure (by ref)"))
  (bind _asbp_player (cast `/Game/InfiniteMatrix/Blueprints/BP_Player` OtherActor))
  (bind _returnvalue (+ (`/Game/InfiniteMatrix/Blueprints/BP_Player.Health` _asbp_player) 0.5))
  (if (>= _returnvalue 1.0)
    (set `/Game/InfiniteMatrix/Blueprints/BP_Player.Health` 1.0 _asbp_player)
    (`ActorComponent.K2_DestroyComponent` (`self.HealPack`))
    (else
      (set `/Game/InfiniteMatrix/Blueprints/BP_Player.Health` _returnvalue _asbp_player)
      (`ActorComponent.K2_DestroyComponent` (`self.HealPack`)))))

(event `self.Enemy.OnComponentBeginOverlap`
  (params (OverlappedComponent :type "PrimitiveComponent Object Reference") (OtherActor :type "Actor Object Reference") (OtherComp :type "PrimitiveComponent Object Reference") (OtherBodyIndex :type Integer) (bFromSweep :type Boolean) (SweepResult :type "HitResult Structure (by ref)"))
  (bind _asbp_player (cast `/Game/InfiniteMatrix/Blueprints/BP_Player` OtherActor)
    (:`then`
      (set `/Game/InfiniteMatrix/Blueprints/BP_Player.Health` (- (`/Game/InfiniteMatrix/Blueprints/BP_Player.Health` _asbp_player) 0.5) _asbp_player)
      (`ActorComponent.K2_DestroyComponent` (`self.Enemy`)))
    (:`CastFailed`
      (bind _asbullet (cast `/Game/InfiniteMatrix/Blueprints/Bullet` OtherActor))
      (`ActorComponent.K2_DestroyComponent` (`self.Enemy`))
      (bind _player (`/Game/InfiniteMatrix/Blueprints/Bullet.Player` _asbullet))
      (bind _score (`/Game/InfiniteMatrix/Blueprints/BP_Player.Score` _player))
      (bind _returnvalue (+ _score 10.0))
      (set `/Game/InfiniteMatrix/Blueprints/BP_Player.Score` _returnvalue _player)
      (if (> _returnvalue (`/Game/InfiniteMatrix/Blueprints/BP_Player.HighScore` _player))
        (set `/Game/InfiniteMatrix/Blueprints/BP_Player.HighScore` _score _player)
        (`self.K2_DestroyActor` _asbullet)))))

(fn `RandomizeHealth`
  (bind _returnvalue (`KismetMathLibrary.RandomIntegerInRange` -200 200))
  (`StaticMeshComponent.SetStaticMesh` (`self.HealPack`) (select `int` (`KismetMathLibrary.RandomIntegerInRange` 0 1) :`0` "/Game/InfiniteMatrix/Meshes/october-pail.october-pail" :`1` null :!type "StaticMesh Object Reference"))
  (`SceneComponent.K2_AddRelativeLocation` (`self.HealPack`) (`KismetMathLibrary.MakeVector` 0.0 (`KismetMathLibrary.Conv_IntToDouble` _returnvalue) (`KismetMathLibrary.Conv_IntToDouble` _returnvalue)) false false))

(fn `RandomizeRat`
  (bind _returnvalue (`KismetMathLibrary.RandomIntegerInRange` -200 200))
  (`StaticMeshComponent.SetStaticMesh` (`self.Enemy`) (select `int` (`KismetMathLibrary.RandomIntegerInRange` 0 1) :`0` "/Game/InfiniteMatrix/Meshes/RATON_MODEL_3D.RATON_MODEL_3D" :`1` null :!type "StaticMesh Object Reference"))
  (`SceneComponent.K2_AddRelativeLocation` (`self.Enemy`) (`KismetMathLibrary.MakeVector` 0.0 (`KismetMathLibrary.Conv_IntToDouble` _returnvalue) (`KismetMathLibrary.Conv_IntToDouble` _returnvalue)) false false))

(fn `RandomizeWall`
  (`StaticMeshComponent.SetStaticMesh` (`self.WallMesh`) (select `int` (`KismetMathLibrary.RandomIntegerInRange` 0 3) :`0` "/Game/InfiniteMatrix/Meshes/SM_Hole_01.SM_Hole_01" :`1` "/Game/InfiniteMatrix/Meshes/SM_Hole_02.SM_Hole_02" :`2` "/Game/InfiniteMatrix/Meshes/SM_Hole_03.SM_Hole_03" :`3` "/Game/InfiniteMatrix/Meshes/SM_Hole_04.SM_Hole_04" :!type "StaticMesh Object Reference"))
  (`SceneComponent.K2_AddLocalRotation` (`self.WallMesh`) (`KismetMathLibrary.MakeRotator` (`KismetMathLibrary.RandomFloatInRange` 0.0 360.0)) false false))

(fn `UserConstructionScript`)